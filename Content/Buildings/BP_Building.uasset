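; BP_Building is a building actor with a door that characters can open and close.
; A box overlap sets or clears NearBuilding on BP_ThirdPersonCharacter.
; OpenDoorSRV forwards to OpenDoorMCST, named as a server-to-multicast pair, which plays a sound and runs a timeline adding incremental yaw to DoorScene.
; InProcess gates toggling but resets on the timeline's first update, alongside the Open flag change, rather than on completion.
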(event OnComponentBeginOverlap(Box)
  (params (OverlappedComponent :type Primitive%20Component%20Object%20Reference) (OtherActor :type Actor%20Object%20Reference) (OtherComp :type Primitive%20Component%20Object%20Reference) (OtherBodyIndex :type Integer) (bFromSweep :type Boolean) (SweepResult :type Hit%20Result%20Structure%20%28by%20ref%29))
  (bind _asbp_third_person_character (Utilities|Casting|CastToBP_ThirdPersonCharacter OtherActor))
  (Variables|/Game/ThirdPerson/Blueprints/BP_ThirdPersonCharacter.BP_ThirdPersonCharacter_C|SetNear_Building _asbp_third_person_character self))

(event OnComponentEndOverlap(Box)
  (params (OverlappedComponent :type Primitive%20Component%20Object%20Reference) (OtherActor :type Actor%20Object%20Reference) (OtherComp :type Primitive%20Component%20Object%20Reference) (OtherBodyIndex :type Integer))
  (bind _asbp_third_person_character (Utilities|Casting|CastToBP_ThirdPersonCharacter OtherActor))
  (Variables|/Game/ThirdPerson/Blueprints/BP_ThirdPersonCharacter.BP_ThirdPersonCharacter_C|SetNear_Building _asbp_third_person_character 0))

(event Custom|Open%20Door%20SRV
  (CallFunction|OpenDoorMCST))

(event Custom|Open%20Door%20MCST
  (if (not (Variables|Default|GetInProcess))
    (Variables|Default|SetInProcess true)
    (if (Variables|Default|GetOpen)
      (Audio|PlaySoundatLocation "/Game/Audio/Close_Door.Close_Door" (Transformation|GetWorldLocation (Variables|Default|GetDoor_Scene)) "0, 0, 0" 1.0 1.0 0.0 0 0 0 0)
      (bind _newtrack_0 (Timeline|Timeline PlayFromStart)
        (:Update
          (Transformation|AddLocalRotation (Variables|Default|GetDoor_Scene) (Math|Rotator|MakeRotator 0.0 0.0 (* _newtrack_0 2.0)) false false)
          (Variables|Default|SetOpen false)
          (Variables|Default|SetInProcess false)))
      (else
        (Audio|PlaySoundatLocation "/Game/Audio/Open_Door.Open_Door" (Transformation|GetWorldLocation (Variables|Default|GetDoor_Scene)) "0, 0, 0" 1.0 1.0 0.0 0 0 0 0)
        (bind _newtrack_0_2 (Timeline|Open_TimeLine PlayFromStart)
          (:Update
            (Transformation|AddLocalRotation (Variables|Default|GetDoor_Scene) (Math|Rotator|MakeRotator 0.0 0.0 (* _newtrack_0_2 -2.0)) false false)
            (Variables|Default|SetOpen true)
            (Variables|Default|SetInProcess false)))))))

(event EventBeginPlay)

(event Collision|EventActorBeginOverlap
  (params (OtherActor :type Actor%20Object%20Reference)))

(event EventTick
  (params (DeltaSeconds :type Float%20%28single-precision%29)))

(fn ConstructionScript)