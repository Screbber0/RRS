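; Inventory component that holds a fixed-size array of item slots, generated on BeginPlay, and refreshes its widget when that widget is valid.
; AddItem looks up the ID in DT_Items, stacks stackable items onto a matching slot or falls back to an empty one, and returns success.
; Both slot searches run without a break, so the last match wins, and stacks have no size cap.
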(event Custom|Update%20Widget
  (bind _widget (Variables|Default|GetWidget))
  (Utilities|IsValid _widget
    (:Is%20Valid
      (Default|Update _widget))))

(event Custom|Create%20Widget%20on%20Client)

(event EventBeginPlay
  (CallFunction|GenerateSlots)
  (CallFunction|UpdateWidget))

(event EventTick
  (params (DeltaSeconds :type Float%20%28single-precision%29)))

(fn GenerateSlots
  (Utilities|Array|Clear (Variables|Default|GetItem_Slots))
  (for _index (range 0 (Variables|Default|GetAmount_Of_Slots))
    (Utilities|Array|Add :TargetArray (Variables|Default|GetItem_Slots))))

(fn SearchEmptySlot
  (bind (_array_element _array_index) (Utilities|Array|ForEachLoopwithBreak (Variables|Default|GetItem_Slots))
    (:LoopBody
      (if (== (.amount _array_element) 0)
        (LocalVariables|SetLocal%20Index _array_index)
        (LocalVariables|SetFounded true)))
    (:Completed
      (return (LocalVariables|GetLocal%20Index) (LocalVariables|GetFounded)))))

(fn SearchSlotforStack
  (params (ID :type Integer))
  (LocalVariables|SetLocal%20ID ID)
  (bind (_array_element _array_index) (Utilities|Array|ForEachLoopwithBreak (Variables|Default|GetItem_Slots))
    (:LoopBody
      (if (== (.id _array_element) (LocalVariables|GetLocal%20ID))
        (LocalVariables|SetLocal%20Index _array_index)
        (LocalVariables|SetFounded true)))
    (:Completed
      (return (LocalVariables|GetLocal%20Index) (LocalVariables|GetFounded)))))

(fn AddItemtoSlot
  (params (Index :type Integer) (Item%20ID :type Integer) (Item%20Amount :type Integer))
  (Utilities|Array|SetArrayElem (Variables|Default|GetItem_Slots) Index (Utilities|Struct|MakeS_ItemSlot Item%20ID (+ Item%20Amount (.amount (Utilities|Array|Get(acopy) (Variables|Default|GetItem_Slots) Index)))))
  (CallFunction|UpdateWidget))

(fn AddItem
  (params (id :type Integer))
  (bind _output_get (LocalVariables|SetLocal%20ID id))
  (bind _returnvalue (Utilities|GetDataTableRow "/Game/Inventory/DT_Items.DT_Items" (Utilities|String|StringToName (Utilities|String|ToString(Integer) _output_get)))
    (:then
      (bind _output_get_2 (LocalVariables|SetLocal%20Item%20Info _returnvalue))
      (if (.stackable (Utilities|Struct|BreakS_ItemStruct _output_get_2))
        (bind (_index _success) (CallFunction|SearchSlotforStack (LocalVariables|GetLocal%20ID)))
        (LocalVariables|SetFounded%20Index _index)
        (if _success
          _
          (else
            (bind (_index_2 _success_2) (CallFunction|SearchEmptySlot :!label _label))
            (LocalVariables|SetFounded%20Index _index_2)
            (if _success_2
              _
              (else
                (return false)))))
        (else
          (goto _label)))
      (CallFunction|AddItemtoSlot (LocalVariables|GetFounded%20Index) (LocalVariables|GetLocal%20ID) 1)
      (return true))
    (:RowNotFound
      (return false))))