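; BP_PickUp is a world pickup actor that represents an inventory item identified by its ID.
; The construction script looks up that ID as a row name in DT_Items and, if found, sets the item mesh from the row.
; AddItem passes the ID to the given character's BPInventoryComponent; the overlap and tick events are unused.
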(event EventBeginPlay)

(event Collision|EventActorBeginOverlap
  (params (OtherActor :type Actor%20Object%20Reference)))

(event EventTick
  (params (DeltaSeconds :type Float%20%28single-precision%29)))

(event EventAddItem
  (params (Character :type BP%20Third%20Person%20Character%20Object%20Reference))
  (Default|AddItem (Variables|/Game/ThirdPerson/Blueprints/BP_ThirdPersonCharacter.BP_ThirdPersonCharacter_C|GetBP_InventoryComponent Character) (Variables|Default|GetID)))

(fn ConstructionScript
  (bind (_row_found _item_struct) (CallFunction|GetItemInfoPerID))
  (if _row_found
    (Components|StaticMesh|SetStaticMesh (Variables|Default|GetItemMesh) (.Mesh (Utilities|Struct|BreakS_ItemStruct _item_struct)))))

(fn GetItemInfoPerID
  (bind _returnvalue (Utilities|GetDataTableRow "/Game/Inventory/DT_Items.DT_Items" (Utilities|String|StringToName (Utilities|String|ToString(Integer) (Variables|Default|GetID))))
    (:then
      (return true _returnvalue))
    (:RowNotFound
      (return false ""))))