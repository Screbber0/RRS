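; BP_Instance, apparently the game instance, loads and saves the player's music and sound volume settings through a BP_SaveGame slot.
; LoadSettings reads saved volumes into its variables and applies them as BP_SoundMix class overrides, or creates the save from current values if none exists.
; SaveSettings writes new volumes to the existing save and applies the same overrides, without updating the instance's own variables.
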(fn LoadSettings
  (bind _returnvalue (SaveGame|DoesSaveGameExist (Variables|Default|GetSave%20Game)))
  (if _returnvalue
    (bind _returnvalue_2 (SaveGame|LoadGamefromSlot (Variables|Default|GetSave%20Game)))
    (bind _asbp_save_game (Utilities|Casting|CastToBP_SaveGame _returnvalue_2))
    (Variables|Default|SetMusic_Value (Variables|/Game/Menu/BP_SaveGame.BP_SaveGame_C|GetMusic_Value _asbp_save_game))
    (Variables|Default|SetSound_Value (Variables|/Game/Menu/BP_SaveGame.BP_SaveGame_C|GetSound_Value _asbp_save_game))
    (Audio|SetSoundMixClassOverride "/Game/Menu/Sounds_Settings/BP_SoundMix.BP_SoundMix" "/Game/Menu/Sounds_Settings/BP_MusicClass.BP_MusicClass" (Variables|Default|GetMusic_Value) 1.0 1.0 true)
    (Audio|SetSoundMixClassOverride "/Game/Menu/Sounds_Settings/BP_SoundMix.BP_SoundMix" "/Game/Menu/Sounds_Settings/BP_SoundClass.BP_SoundClass" (Variables|Default|GetSound_Value) 1.0 1.0 true)
    (else
      (bind _returnvalue_3 (SaveGame|CreateSaveGameObject "/Game/Menu/BP_SaveGame.BP_SaveGame_C"))
      (bind _output_get (Variables|Default|SetBP%20Save%20Data _returnvalue_3))
      (Variables|/Game/Menu/BP_SaveGame.BP_SaveGame_C|SetMusic_Value _output_get (Variables|Default|GetMusic_Value))
      (Variables|/Game/Menu/BP_SaveGame.BP_SaveGame_C|SetSound_Value _output_get (Variables|Default|GetSound_Value))
      (SaveGame|SaveGametoSlot _output_get (Variables|Default|GetSave%20Game)))))

(fn SaveSettings
  (params (Sound_Value :type Float%20%28double-precision%29) (Music_Value :type Float%20%28double-precision%29))
  (bind _returnvalue (SaveGame|LoadGamefromSlot (Variables|Default|GetSave%20Game)))
  (bind _asbp_save_game (Utilities|Casting|CastToBP_SaveGame _returnvalue))
  (bind _output_get (Variables|/Game/Menu/BP_SaveGame.BP_SaveGame_C|SetSound_Value _asbp_save_game Sound_Value))
  (Audio|SetSoundMixClassOverride "/Game/Menu/Sounds_Settings/BP_SoundMix.BP_SoundMix" "/Game/Menu/Sounds_Settings/BP_SoundClass.BP_SoundClass" _output_get 1.0 1.0 true)
  (bind _output_get_2 (Variables|/Game/Menu/BP_SaveGame.BP_SaveGame_C|SetMusic_Value _asbp_save_game Music_Value))
  (Audio|SetSoundMixClassOverride "/Game/Menu/Sounds_Settings/BP_SoundMix.BP_SoundMix" "/Game/Menu/Sounds_Settings/BP_MusicClass.BP_MusicClass" _output_get_2 1.0 1.0 true)
  (SaveGame|SaveGametoSlot _asbp_save_game (Variables|Default|GetSave%20Game)))